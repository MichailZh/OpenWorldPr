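; Zombie enemy character that detects, attacks and takes damage from the TestFpp player.
; PawnSensing sight or repeated noises trigger a scream and set EnemyFound; lesser noises pause it, then ZombieController resumes patrolling.
; Bone-based damage makes headshots lethal and leg hits cause crawling, while death ragdolls it and drops randomly chosen AK74 or sniper ammo.
; A Scan line trace tracks time without a target, and sphere overlap deals melee damage while attacking.
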(event `self.PawnSensing.OnSeePawn`
  (params (Pawn :type "Pawn Object Reference"))
  ;[1 1 1] Sight
  (cast `/Game/Character/MainCharFPP/TestFpp` Pawn)
  (if (not (`self.EnemyFound`))
    (if (not (`self.Crawling`)) :!label _label
      (`/Engine/EditorBlueprintResources/StandardMacros.DoOnce` false :!label _label_2
        (:`Completed`
          (`MovementComponent.StopMovementImmediately` (`self.CharacterMovement`))
          (set `self.WaitStart` true)
          (`self.PlayAnimMontage` "/Game/AI/Zombie/Animations/zombie_Skeleton_Montage.zombie_Skeleton_Montage")
          (`KismetSystemLibrary.Delay` 2.7)
          (set `self.WaitStart` false)))))
  (set `self.EnemyFound` true)
  (set `self.Time` 0)
  (`self.ResetScream`))

(event `ResetScream`
  ;[1 1 1] Sight
  (goto _label_2 :!via `Reset`))

(event `/Game/AI/ActiveAI/AI2/DamageIF.TakingDamage`
  (params (BoneName :type Name) (Damage :type "Float (single-precision)"))
  ;[1 1 1] Damage
  (if (== BoneName "Head")
    (set `self.CurrentHealth` 0.0 :!label _label_3)
    (else
      (set `self.CurrentHealth` (- (`self.CurrentHealth`) Damage))
      (if (or (== BoneName "LeftLeg") (== BoneName "LeftFoot") (== BoneName "LeftToeBase") (== BoneName "RightLeg") (== BoneName "RightFoot") (== BoneName "RightToeBase") (== BoneName "LeftUpLeg") (== BoneName "RightUpLeg"))
        (if (<= (`self.CurrentHealth`) 0.0)
          (goto _label_3)
          (else
            (`/Engine/EditorBlueprintResources/StandardMacros.DoOnce` false
              (:`Completed`
                (set `self.Laying` true)
                (set `CharacterMovementComponent.MaxWalkSpeed` 0.0 (`self.CharacterMovement`))
                (`self.PlayAnimMontage` "/Game/AI/Zombie/Animations/Zombie_Dying_Montage.Zombie_Dying_Montage")
                (set `self.Crawling` true)
                (`KismetSystemLibrary.Delay` 2.367)
                (set `self.Laying` false)))))
        (elif (not (`self.Crawling`))
          (`self.PlayAnimMontage` (`self.CurrentMontage`))))
      (set `self.EnemyFound` true)
      (set `self.Time` 0)))
  (if (<= (`self.CurrentHealth`) 0.0)
    (set `self.CurrentHealth` 0.0)
    (set `self.IsDead?` true)
    (`self.Drop`)
    (`SkeletalMeshComponent.SetAllBodiesSimulatePhysics` (`self.Mesh`) true)
    (`PrimitiveComponent.SetCollisionEnabled` (`self.Mesh`) "QueryAndPhysics")
    (`CharacterMovementComponent.DisableMovement` (`self.CharacterMovement`))
    (`KismetSystemLibrary.Delay` 3.0)
    (`self.K2_DestroyActor`)))

(event `self.PawnSensing.OnHearNoise`
  (params (Instigator :type "Pawn Object Reference") (Location :type "Vector Structure (by ref)") (Volume :type "Float (single-precision)"))
  (if (>= (`self.IsHeard`) 5)
    (goto _label)
    (else
      (`MovementComponent.StopMovementImmediately` (`self.CharacterMovement`))
      (bind _result (`/Engine/EditorBlueprintResources/StandardMacros.IncrementInt` (`self.IsHeard`))
        (:`  `
          (set `self.IsHeard` _result)
          (set `self.WaitStart` true)
          (`KismetSystemLibrary.RetriggerableDelay` 2.0)
          (set `self.WaitStart` false)
          (set `self.IsHeard` 0)
          (if (not (`self.EnemyFound`))
            (`/Game/AI/Zombie/ZombieController.Patroling` (cast `/Game/AI/Zombie/ZombieController` (`self.GetController`) :!pure true))))))))

(event `Drop`
  ;[1 1 1] Drop
  (`/Engine/EditorBlueprintResources/StandardMacros.DoOnce` false
    (:`Completed`
      (`self.DropAmmo`))))

(event `self.ReceiveBeginPlay`
  ;[1 1 1] Begin
  (set `CharacterMovementComponent.MaxWalkSpeed` 125.0 (`self.CharacterMovement`))
  (if (== (`KismetMathLibrary.RandomIntegerInRange` 0 1) 0)
    (set `self.AmmoInfo` "NewEnumerator0")
    (else
      (set `self.AmmoInfo` "NewEnumerator1"))))

(event `Scan`
  (bind _arrow2 (`self.Arrow2`))
  (bind _returnvalue (`SceneComponent.K2_GetComponentLocation` _arrow2))
  ;[1 1 1] Scan
  (bind (_outhit _returnvalue_2) (`KismetSystemLibrary.LineTraceSingle` _returnvalue (+ (* (`SceneComponent.GetForwardVector` _arrow2) 50000.0) _returnvalue) "TraceTypeQuery1" true (`|MakeArray` self :!type "Actor Object Reference") "None" true (struct :`R` 1.0 :`B` 0.118228 :`A` 1.0)))
  (if _returnvalue_2
    _
    (else
      _))
  (if (`KismetSystemLibrary.DoesImplementInterface` (`.HitActor` (`GameplayStatics.BreakHitResult` _outhit)) "/Game/AI/ActiveAI/AI2/DamageIF.DamageIF_C")
    (set `self.Active` true)
    (set `self.Time` 0)
    (set `self.StopWatch` false)
    (else
      (set `self.Active` false)
      (bind _output_get (set `self.StopWatch` true))
      (if _output_get
        (`KismetSystemLibrary.Delay` 1.0)
        (bind _result (`/Engine/EditorBlueprintResources/StandardMacros.IncrementInt` (`self.Time`))
          (:`  `
            (set `self.Time` _result)))))))

(event `self.ReceiveTick`
  (params (DeltaSeconds :type "Float (single-precision)"))
  ;[1 1 1] Scan
  (if (!= (`KismetMathLibrary.VSize` (`self.GetVelocity`)) 0.0)
    (set `self.WaitStart` false)))

(event `self.Sphere.OnComponentBeginOverlap`
  (params (OverlappedComponent :type "PrimitiveComponent Object Reference") (OtherActor :type "Actor Object Reference") (OtherComp :type "PrimitiveComponent Object Reference") (OtherBodyIndex :type Integer) (bFromSweep :type Boolean) (SweepResult :type "HitResult Structure (by ref)"))
  (bind _astest_fpp (cast `/Game/Character/MainCharFPP/TestFpp` OtherActor)
    (:`then`
      _)
    (:`CastFailed`
      _))
  (if (== OtherActor _astest_fpp)
    (if (`self.Attacking`)
      (if (not (`self.HitSchon`))
        (message `/Game/AI/ActiveAI/AI2/DamageIF.TakingDamage` _astest_fpp "None" 20.0)
        (set `self.HitSchon` true)))))

(fn `DropAmmo`
  (returns (ReturnValue :type "/Game/Character/Interactables/Objects/Ammo/BP_BaseAmmo Object Reference"))
  (bind _ammomaster (`self.AmmoMaster`))
  (bind _returnvalue (`SceneComponent.K2_GetComponentToWorld` (`self.Arrow1`)))
  (switch `/Game/Character/Interactables/Objects/Ammo/AmmoType` (`self.AmmoInfo`)
    (:`NewEnumerator0`
      (set `self.AmmoMaster` "/Game/Character/Interactables/Objects/Ammo/AmmoAk74.AmmoAk74_C")
      (bind _returnvalue_2 (`|SpawnActorFromClass` _ammomaster _returnvalue "Undefined" "OverrideRootScale" null null))
      (return _returnvalue_2))
    (:`NewEnumerator1`
      (set `self.AmmoMaster` "/Game/Character/Interactables/Objects/Ammo/AmmoSniper.AmmoSniper_C")
      (bind _returnvalue_3 (`|SpawnActorFromClass` _ammomaster _returnvalue "Undefined" "OverrideRootScale" null null))
      (return _returnvalue_3))))

(fn `UserConstructionScript`)