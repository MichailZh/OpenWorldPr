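; BP_CharRecorder is a character stand-in, apparently for scene capture, that mirrors the player's equipped weapons on its skeletal mesh.
; On BeginPlay it passes itself to the TestFpp player character.
; EquipItem spawns a copy of Auto or Sniper weapons at their holstered (unequip) socket, storing it as RifleRef or SniperRef.
; UnequipItem picks by slot rather than type, destroying both that copy and the passed-in weapon.
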(event `self.ReceiveBeginPlay`
  (bind _astest_fpp (cast `/Game/Character/MainCharFPP/TestFpp` (`GameplayStatics.GetPlayerCharacter` 0)))
  (message `/Game/Character/Interactables/Objects/BPI_PassReferences.PassRef` _astest_fpp self))

(event `/Game/Character/Interactables/Objects/BPI_PassReferences.EquipItem`
  (params (ItemInfo :type "/Game/Character/Interactables/Objects/FItemInfo Structure") (WeaponInfo :type "/Game/Character/Interactables/Objects/Weapon/WeaponInfo Structure") (Weapon :type "Actor Object Reference"))
  (`self.AttachItem` ItemInfo Weapon))

(event `/Game/Character/Interactables/Objects/BPI_PassReferences.UnequipItem`
  (params (ItemInfo :type "/Game/Character/Interactables/Objects/FItemInfo Structure") (Weaponinfo :type "/Game/Character/Interactables/Objects/Weapon/WeaponInfo Structure") (Weapon :type "Actor Object Reference"))
  (`self.UnattachItem` ItemInfo Weapon))

(fn `AttachItem`
  (params (ItemInfo :type "/Game/Character/Interactables/Objects/FItemInfo Structure") (Weapon :type "Actor Object Reference"))
  (bind _skeletalmesh (`self.SkeletalMesh`))
  (bind _output_get (set `self.BaseWeaponMaster` Weapon))
  (bind _asbp_base_weapon (cast `/Game/Character/Interactables/Objects/Weapon/BP_BaseWeapon` _output_get))
  (bind (_itemtype _itemclass _clipsize _currentammo _maxammo _damage _equipsocketname _unequipsocketname) (break `/Game/Character/Interactables/Objects/Weapon/WeaponInfo` (`/Game/Character/Interactables/Objects/Weapon/BP_BaseWeapon.ItemInfo` _asbp_base_weapon)))
  (switch `/Game/Character/Interactables/Objects/Weapon/OruzhieType` _itemtype
    (:`NewEnumerator1`
      (bind _returnvalue (`|SpawnActorFromClass` _itemclass (`SceneComponent.GetSocketTransform` _skeletalmesh _unequipsocketname "RTS_World") "Undefined" "OverrideRootScale" null null))
      (bind _output_get_2 (set `self.RifleRef` _returnvalue))
      (`self.K2_AttachToComponent` _output_get_2 (`self.SkeletalMesh`) _unequipsocketname "SnapToTarget" "SnapToTarget" "KeepWorld" true))
    (:`NewEnumerator2`
      (bind _returnvalue_2 (`|SpawnActorFromClass` _itemclass (`SceneComponent.GetSocketTransform` _skeletalmesh _unequipsocketname "RTS_World") "Undefined" "OverrideRootScale" null null))
      (bind _output_get_3 (set `self.SniperRef` _returnvalue_2))
      (`self.K2_AttachToComponent` _output_get_3 (`self.SkeletalMesh`) _unequipsocketname "SnapToTarget" "SnapToTarget" "KeepWorld" true))))

(fn `UnattachItem`
  (params (ItemInfo :type "/Game/Character/Interactables/Objects/FItemInfo Structure") (Weapon :type "Actor Object Reference"))
  (switch `/Game/Character/Interactables/Objects/ISlotType` (`.ItemSlot_24_CF369CA24348A2FCC3AFDF97B943B020` (break `/Game/Character/Interactables/Objects/FItemInfo` ItemInfo))
    (:`NewEnumerator7`
      (`self.K2_DestroyActor` (`self.RifleRef`))
      (`self.K2_DestroyActor` Weapon))
    (:`NewEnumerator8`
      (`self.K2_DestroyActor` Weapon)
      (`self.K2_DestroyActor` (`self.SniperRef`)))))

(fn `UserConstructionScript`)