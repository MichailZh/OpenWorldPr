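; Item inspection actor that spawns and removes the item the player inspects.
; On BeginPlay it registers itself with the TestFpp player character.
; InspectItem spawns the ItemInfo class at its StaticMesh transform, stores the instance and sets the player's IsInspecting flag.
; UnInspectItem removes the inspect widget reached through the player's inventory reference, clears the flag and destroys the spawned item.
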(event `self.ReceiveBeginPlay`
  (bind _astest_fpp (cast `/Game/Character/MainCharFPP/TestFpp` (`GameplayStatics.GetPlayerCharacter` 0)))
  (`/Game/Character/Interactables/Objects/BP_BaseItem.PassObjectRef` _astest_fpp self))

(event `/Game/Character/Interactables/Objects/BPI_Inventory.InspectItem`
  (params (ItemInfo :type "/Game/Character/Interactables/Objects/FItemInfo Structure"))
  (bind _returnvalue (`|SpawnActorFromClass` (`.ItemClass_14_90984E5341269B8FD36FBDA1A0B704D0` (break `/Game/Character/Interactables/Objects/FItemInfo` ItemInfo)) (`SceneComponent.K2_GetComponentToWorld` (`self.StaticMesh`)) "Undefined" "OverrideRootScale" null null))
  (set `self.InspectedObject` _returnvalue)
  (set `/Game/Character/MainCharFPP/TestFpp.IsInspecting` true (stale `self.ReceiveBeginPlay` _astest_fpp)))

(event `/Game/Character/Interactables/Objects/BPI_Inventory.UnInspectItem`
  (`Widget.RemoveFromParent` (`/Game/Character/Interactables/Objects/UI/UI_Inventory.InspectRef` (`/Game/Character/MainCharFPP/TestFpp.InventRef` (stale `self.ReceiveBeginPlay` _astest_fpp))))
  (set `/Game/Character/MainCharFPP/TestFpp.IsInspecting` false (stale `self.ReceiveBeginPlay` _astest_fpp))
  (`self.K2_DestroyActor` (`self.InspectedObject`)))

(fn `UserConstructionScript`)