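; BP_WeaponSpawner spawns random items from the ItemToSpawn class list inside its Box volume when play begins.
; AttemptToSpawn calls SpawnItems unless CurrentItem is valid, in which case it only prints a debug string.
; SpawnItems loops once per list entry, placing actors at random box points and keeping the latest as CurrentItem.
; Its repeat check is unreliable because the checked, spawned and stored indices are separate random rolls.
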(event `self.ReceiveBeginPlay`
  (`self.AttemptToSpawn`))

(fn `AttemptToSpawn`
  (`/Engine/EditorBlueprintResources/StandardMacros.IsValid` (`self.CurrentItem`)
    (:`Is Valid`
      (`KismetSystemLibrary.PrintString` "Hello"))
    (:`Is Not Valid`
      (`self.SpawnItems`))))

(fn `SpawnItems`
  (bind _returnvalue (`KismetMathLibrary.RandomIntegerInRange` 0 (- (`KismetArrayLibrary.Array_Length` (`self.ItemToSpawn`)) 1)))
  (for _ (range 1 (+ (`KismetArrayLibrary.Array_Length` (`self.ItemToSpawn`)) 1))
    (bind _output_get (set `self.ItemIndex` _returnvalue))
    (if (not (== _output_get (`self.PreviousIndex`)))
      (bind _returnvalue_2 (`|SpawnActorFromClass` (`|GetArrayItem` (`self.ItemToSpawn`) _returnvalue) (`KismetMathLibrary.MakeTransform` (`KismetMathLibrary.RandomPointInBoundingBox` (`SceneComponent.K2_GetComponentLocation` (`self.Box`)) (`BoxComponent.BoxExtent` (`self.Box`))) (`self.K2_GetActorRotation`)) "Undefined" "OverrideRootScale" null null))
      (set `self.PreviousIndex` _returnvalue)
      (set `self.CurrentItem` _returnvalue_2))))

(fn `UserConstructionScript`)