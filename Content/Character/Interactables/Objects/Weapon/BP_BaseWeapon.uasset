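; Base weapon actor for the TestFpp character, handling overlap outline highlighting, automatic fire, ammo and reloading.
; A looping timer fires camera-centered line traces that damage DamageIF actors and destructibles, then spawns a muzzle projectile aimed at the impact, plus a decal.
; Each shot plays shake, montage and sound, applies random recoil by movement state, and decrements WeaponInfo and the character's rifle or sniper counters.
; Releasing fire auto-reloads an empty clip from reserve ammo.
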(event `self.IteractableArea.OnComponentBeginOverlap`
  (params (OverlappedComponent :type "PrimitiveComponent Object Reference") (OtherActor :type "Actor Object Reference") (OtherComp :type "PrimitiveComponent Object Reference") (OtherBodyIndex :type Integer) (bFromSweep :type Boolean) (SweepResult :type "HitResult Structure (by ref)"))
  ;[1 1 1] Input
  (bind _astest_fpp (cast `/Game/Character/MainCharFPP/TestFpp` OtherActor))
  (set `self.Ref_0` _astest_fpp)
  (`PrimitiveComponent.SetRenderCustomDepth` (`self.SkeletalMesh`) true))

(event `self.IteractableArea.OnComponentEndOverlap`
  (params (OverlappedComponent :type "PrimitiveComponent Object Reference") (OtherActor :type "Actor Object Reference") (OtherComp :type "PrimitiveComponent Object Reference") (OtherBodyIndex :type Integer))
  ;[1 1 1] Input
  (bind _astest_fpp (cast `/Game/Character/MainCharFPP/TestFpp` OtherActor))
  (set `self.Ref_0` _astest_fpp)
  (`PrimitiveComponent.SetRenderCustomDepth` (`self.SkeletalMesh`) false))

(event `Off`
  ;[1 1 1] Input
  (`PrimitiveComponent.SetRenderCustomDepth` (`self.SkeletalMesh`) false)
  (`ActorComponent.K2_DestroyComponent` (`self.IteractableArea`))
  (`self.DisableInput` (`GameplayStatics.GetPlayerController` 0)))

(event `StartFire`
  (bind _returnvalue (`GameplayStatics.GetPlayerCameraManager` 0))
  (bind _ref_0 (`self.Ref_0`))
  (bind _returnvalue_2 (`self.K2_GetActorLocation` _returnvalue))
  (bind _skeletalmesh (`/Game/Character/Interactables/Objects/Weapon/BP_BaseWeapon.SkeletalMesh` (`/Game/Character/MainCharFPP/TestFpp.SniperBP1` (`self.Ref_0`))))
  (bind _skeletalmesh_2 (`/Game/Character/Interactables/Objects/Weapon/BP_BaseWeapon.SkeletalMesh` (`/Game/Character/MainCharFPP/TestFpp.RifleBP1` (`self.Ref_0`))))
  (bind _returnvalue_3 (`SceneComponent.GetSocketLocation` _skeletalmesh (`SkinnedMeshComponent.GetSocketBoneName` _skeletalmesh "Muzzle")))
  (bind _returnvalue_4 (`SceneComponent.GetSocketLocation` _skeletalmesh_2 (`SkinnedMeshComponent.GetSocketBoneName` _skeletalmesh_2 "Muzzle")))
  ;[1 1 1] Shot
  (bind _returnvalue_5 (`KismetSystemLibrary.K2_SetTimerDelegate` (delegate `Shot`) (`.ShootSpeed_29_04FE17954F834FBDA91E65801E92AEB9` (break `/Game/Character/Interactables/Objects/Weapon/WeaponInfo` (`self.WeaponInfo`))) true))
  (if (`/Game/Character/MainCharFPP/TestFpp.Is Combating?` (`self.Ref_0`)) :!label _label
    (if (not (<= (`.CurrentAmmo_11_77294F7E436BCFA25A02669793C1006D` (break `/Game/Character/Interactables/Objects/Weapon/WeaponInfo` (`self.WeaponInfo`))) 0))
      (bind _astest_fpp_anim (cast `/Game/Character/MainCharFPP/TestFppAnim` (`SkeletalMeshComponent.GetAnimInstance` (`Character.Mesh` (`self.Ref_0`)))))
      (`GameplayStatics.PlayWorldCameraShake` "/Game/Character/MainCharFPP/BP_CameraShake.BP_CameraShake_C" (`self.K2_GetActorLocation` (`self.Ref_0`)) 0.0 87.0)
      (`AnimInstance.Montage_Play` _astest_fpp_anim "/Game/Character/Animations/Fire_Rifle_Ironsights_Montage.Fire_Rifle_Ironsights_Montage" 1.0 "MontageLength" 0.0 true)
      (`GameplayStatics.PlaySound2D` (`.Sound_34_E88FE577483300B9533513A049E91D65` (break `/Game/Character/Interactables/Objects/Weapon/WeaponInfo` (`self.WeaponInfo`))) 1.0 1.0 0.0 null null)
      (bind (_outhit _returnvalue_6) (`KismetSystemLibrary.LineTraceSingle` _returnvalue_2 (+ _returnvalue_2 (* (`self.GetActorForwardVector` _returnvalue) 15000.0)) "TraceTypeQuery2" true (`|MakeArray` (`self.Ref_0`) :!type "Actor Object Reference")))
      (`self.Recoil`
        (:`then`
          _)
        (:`then2`
          _))
      (if _returnvalue_6
        _
        (else
          _))
      (bind (_bblockinghit _binitialoverlap _time _distance _location _impactpoint _normal _impactnormal _physmat _hitactor _hitcomponent _hitbonename _hititem _faceindex _tracestart _traceend) (`GameplayStatics.BreakHitResult` _outhit))
      (bind _output_get (set `self.HitLocation` _location))
      (bind _asdestructible_actor (cast `DestructibleActor` _hitactor)
        (:`then`
          (`DestructibleComponent.ApplyRadiusDamage` (`DestructibleActor.DestructibleComponent` _asdestructible_actor) 200.0 _output_get 0.05 5000.0 false))
        (:`CastFailed`
          _))
      (`self.AmmoCulc`)
      (if (`KismetSystemLibrary.DoesImplementInterface` _hitactor "/Game/AI/ActiveAI/AI2/DamageIF.DamageIF_C")
        (message `/Game/AI/ActiveAI/AI2/DamageIF.TakingDamage` _hitactor _hitbonename (`.Damage_16_CE1352594236CBF13E60C09FC37B608E` (break `/Game/Character/Interactables/Objects/Weapon/WeaponInfo` (`self.WeaponInfo`)))))
      (if (`/Game/Character/MainCharFPP/TestFpp.EquipRifle` _ref_0)
        (`|SpawnActorFromClass` "/Game/Character/Interactables/Objects/Weapon/Projectile.Projectile_C" (`KismetMathLibrary.MakeTransform` _returnvalue_4 (`KismetMathLibrary.FindLookAtRotation` _returnvalue_4 (`KismetMathLibrary.SelectVector` _impactpoint _traceend _returnvalue_6))) "Undefined" "OverrideRootScale" null null)
        (bind (_returnvalue_roll _returnvalue_pitch _returnvalue_yaw) (`KismetMathLibrary.BreakRotator` (`KismetMathLibrary.MakeRotFromX` _normal)))
        (`GameplayStatics.SpawnDecalAtLocation` "/Game/Character/MaterialsCustom/BH.BH" (10.0 10.0 10.0) _output_get (`KismetMathLibrary.MakeRotator` (+ _returnvalue_roll 0.0) (+ _returnvalue_pitch 180.0) (+ _returnvalue_yaw 0.0)) 180.0 :!label _label_2)
        (elif (`/Game/Character/MainCharFPP/TestFpp.EquipSniper` _ref_0)
          (`|SpawnActorFromClass` "/Game/Character/Interactables/Objects/Weapon/Projectile.Projectile_C" (`KismetMathLibrary.MakeTransform` _returnvalue_3 (`KismetMathLibrary.FindLookAtRotation` _returnvalue_3 (`KismetMathLibrary.SelectVector` _impactpoint _traceend _returnvalue_6))) "Undefined" "OverrideRootScale" null null)
          (goto _label_2))))))

(event `StopFire`
  ;[1 1 1] Shot
  (`KismetSystemLibrary.K2_ClearAndInvalidateTimerHandle` (stale `StartFire` _returnvalue_5)))

(event `Shot`
  ;[1 1 1] Shot
  (goto _label))

(event `FirePress`
  ;[1 1 1] Reload
  (set `self.CanFire?` true)
  (if (not (`self.IsReloading?`))
    (`self.StartFire`)))

(event `FireRelease`
  ;[1 1 1] Reload
  (set `self.CanFire?` false)
  (`self.StopFire`)
  (`self.AutoReload`))

(event `AutoReload`
  ;[1 1 1] Reload
  (if (== (`.CurrentAmmo_11_77294F7E436BCFA25A02669793C1006D` (break `/Game/Character/Interactables/Objects/Weapon/WeaponInfo` (`self.WeaponInfo`))) 0)
    (if (== (`.MaxAmmo_15_9D4DDDDC4658FE52F72BF4A08B307360` (break `/Game/Character/Interactables/Objects/Weapon/WeaponInfo` (`self.WeaponInfo`))) 0)
      (`GameplayStatics.PlaySound2D` "/Game/Sounds/386037__taramg__riflereload001.386037__taramg__riflereload001" 1.0 1.0 0.0 null null)
      (else
        (set `self.IsReloading?` true)
        (`self.Reloading`)
        (`GameplayStatics.PlaySound2D` "/Game/Sounds/363167__samsterbirdies__mag-reload.363167__samsterbirdies__mag-reload" 1.0 1.0 0.0 null null)
        (`KismetSystemLibrary.Delay` 2.0)
        (set `self.IsReloading?` false)))))

(event `Reloading`
  (bind (_itemtype _itemclass _clipsize _currentammo) (break `/Game/Character/Interactables/Objects/Weapon/WeaponInfo` (`self.WeaponInfo`)))
  ;[1 1 1] Reload
  (if (== (`.MaxAmmo_15_9D4DDDDC4658FE52F72BF4A08B307360` (break `/Game/Character/Interactables/Objects/Weapon/WeaponInfo` (`self.WeaponInfo`))) 0)
    _
    (elif (not (== _clipsize _currentammo))
      (bind _output_get (set `self.IsReloading?` true))
      (if _output_get
        (`self.WeaponReload`)
        (`GameplayStatics.PlaySound2D` "/Game/Sounds/363167__samsterbirdies__mag-reload.363167__samsterbirdies__mag-reload" 1.0 1.0 0.0 null null)
        (`KismetSystemLibrary.Delay` 2.0)
        (set `self.IsReloading?` false)))))

(event `WeaponReload`
  (bind _weaponinfo (`self.WeaponInfo`))
  (bind _neededammo (`self.NeededAmmo`))
  (bind (_itemtype _itemclass _clipsize _currentammo) (break `/Game/Character/Interactables/Objects/Weapon/WeaponInfo` (`self.WeaponInfo`)))
  (bind (_itemtype_2 _itemclass_2 _clipsize_2 _currentammo_2 _maxammo) (break `/Game/Character/Interactables/Objects/Weapon/WeaponInfo` (`self.WeaponInfo`)))
  (bind (_itemtype_3 _itemclass_3 _clipsize_3 _currentammo_3 _maxammo_2) (break `/Game/Character/Interactables/Objects/Weapon/WeaponInfo` (`self.WeaponInfo`)))
  ;[1 1 1] Reload
  (if (not (`self.CanFire?`))
    (`Character.PlayAnimMontage` (`self.Ref_0`) "/Game/AnimStarterPack/ReloadMontage.ReloadMontage" 1.0 "None")
    (if (> (`.MaxAmmo_15_9D4DDDDC4658FE52F72BF4A08B307360` (break `/Game/Character/Interactables/Objects/Weapon/WeaponInfo` (`self.WeaponInfo`))) 0)
      (set `self.NeededAmmo` (- _clipsize _currentammo))
      (if (<= _maxammo _neededammo)
        (setmembers `/Game/Character/Interactables/Objects/Weapon/WeaponInfo` :`StructRef` _weaponinfo :`CurrentAmmo` (+ _currentammo_3 _maxammo_2))
        (setmembers `/Game/Character/Interactables/Objects/Weapon/WeaponInfo` :`StructRef` _weaponinfo :`MaxAmmo` 0)
        (else
          (setmembers `/Game/Character/Interactables/Objects/Weapon/WeaponInfo` :`StructRef` _weaponinfo :`MaxAmmo` (- _maxammo _neededammo))
          (setmembers `/Game/Character/Interactables/Objects/Weapon/WeaponInfo` :`StructRef` _weaponinfo :`CurrentAmmo` (`.ClipSize_26_8245B85B4C50D1B8C0E4C7801BBABD36` (break `/Game/Character/Interactables/Objects/Weapon/WeaponInfo` (`self.WeaponInfo`)))))))))

(fn `UserConstructionScript`
  (bind (_weaponinfo_itemtype _weaponinfo_itemclass _weaponinfo_clipsize _weaponinfo_currentammo _weaponinfo_maxammo _weaponinfo_damage _weaponinfo_equipsocketname _weaponinfo_unequipsocketname _weaponinfo_shootspeed _weaponinfo_sound) (break `/Game/Character/Interactables/Objects/Weapon/WeaponInfo` (`self.WeaponInfo`)))
  (`parent.UserConstructionScript`)
  (set `self.WeaponInfo` (make `/Game/Character/Interactables/Objects/Weapon/WeaponInfo` _weaponinfo_itemtype (`GameplayStatics.GetObjectClass` self) _weaponinfo_clipsize _weaponinfo_currentammo _weaponinfo_maxammo _weaponinfo_damage _weaponinfo_equipsocketname _weaponinfo_unequipsocketname _weaponinfo_shootspeed _weaponinfo_sound)))