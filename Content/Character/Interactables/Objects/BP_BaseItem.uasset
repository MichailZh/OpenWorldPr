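; Base interactable item that the player picks up into their inventory when space is available.
; Construction script stamps the actor's own class into its ItemInfo struct.
; On Interaction, rifle or sniper slot items first unequip and drop the player's existing weapon in that slot and refresh the inventory UI.
; It then messages the instigator to pick up, handing one item type to the player and destroying others, recalculating bullets for another type.
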(event `/Game/Character/Interactables/Objects/BPI_Iteract.Interaction`
  (params (Insrigator :type "/Game/Character/MainCharFPP/TestFpp Object Reference"))
  (bind _iteminfo_0 (`self.ItemInfo_0`))
  (bind _ref (`self.Ref`))
  (bind _iteminfo_0_2 (`self.ItemInfo_0`))
  (bind _iteminfo_0_3 (`self.ItemInfo_0`))
  (bind _ref_2 (`self.Ref`))
  (bind _ref_3 (`self.Ref`))
  (bind _ref_4 (`self.Ref`))
  (bind _itemtype (break `/Game/Character/Interactables/Objects/FItemInfo` (`self.ItemInfo_0`)))
  (bind (_itemtype_2 _itemname _itemimage _itemclass _itemindex _itemslot) (break `/Game/Character/Interactables/Objects/FItemInfo` (`self.ItemInfo_0`)))
  (bind _sniperbp1 (`/Game/Character/MainCharFPP/TestFpp.SniperBP1` _ref))
  (bind _riflebp1 (`/Game/Character/MainCharFPP/TestFpp.RifleBP1` _ref_3))
  (bind _refrecchar (`/Game/Character/MainCharFPP/TestFpp.RefRecChar` _ref_4))
  (bind _astest_fpp (cast `/Game/Character/MainCharFPP/TestFpp` (`GameplayStatics.GetPlayerCharacter` 0)))
  (bind _output_get (set `self.Ref` _astest_fpp))
  (if (`/Game/Character/MainCharFPP/TestFpp.Has Space in Inventory` _astest_fpp)
    (if (`|EnumEquality` _itemslot "NewEnumerator7")
      (if (`KismetSystemLibrary.IsValid` (`/Game/Character/MainCharFPP/TestFpp.RifleBP1` _output_get))
        (if (`/Game/Character/MainCharFPP/TestFpp.Is Combating?` (`self.Ref`))
          (`/Game/Character/MainCharFPP/TestFpp.Equip` _ref_4))
        (`/Game/Character/MainCharFPP/TestFpp.RemoveFromEq` _ref_4 _iteminfo_0)
        (message `/Game/Character/Interactables/Objects/BPI_Inventory.DropWeapon` _ref_3 _riflebp1 _iteminfo_0)
        (message `/Game/Character/Interactables/Objects/BPI_PassReferences.UnequipItem` _refrecchar _iteminfo_0 (struct) _riflebp1)
        (`/Game/Character/MainCharFPP/TestFpp.StartRefresh` _ref_2)
        (`/Game/Character/MainCharFPP/TestFpp.RefreshInvent` _ref_2)
        (`/Game/Character/MainCharFPP/TestFpp.RefreshEq` _ref_2))
      (elif (`|EnumEquality` _itemslot "NewEnumerator8")
        (if (`KismetSystemLibrary.IsValid` (`/Game/Character/MainCharFPP/TestFpp.SniperBP1` (`self.Ref`)))
          (if (`/Game/Character/MainCharFPP/TestFpp.Is Combating?` (`self.Ref`))
            (`/Game/Character/MainCharFPP/TestFpp.Equip` _ref_4))
          (`/Game/Character/MainCharFPP/TestFpp.RemoveFromEq` _ref_4 _iteminfo_0_2)
          (message `/Game/Character/Interactables/Objects/BPI_Inventory.DropWeapon` _ref _sniperbp1 _iteminfo_0)
          (message `/Game/Character/Interactables/Objects/BPI_PassReferences.UnequipItem` _refrecchar _iteminfo_0_2 (struct) _sniperbp1)
          (`/Game/Character/MainCharFPP/TestFpp.StartRefresh` _ref)
          (`/Game/Character/MainCharFPP/TestFpp.RefreshInvent` _ref)
          (`/Game/Character/MainCharFPP/TestFpp.RefreshEq` _ref))))
    (message `/Game/Character/Interactables/Objects/BPI_Iteract.PickUpItem` Insrigator _iteminfo_0_3 self)
    (if (== _itemtype 4)
      (`/Game/Character/MainCharFPP/TestFpp.PickUp` (`self.Ref`) self)
      (elif (`|EnumEquality` _itemtype "NewEnumerator1")
        (`/Game/Character/MainCharFPP/TestFpp.CalculateBullets` (`self.Ref`) _iteminfo_0_3)
        (`self.K2_DestroyActor`)
        (else
          (`self.K2_DestroyActor`))))))

(fn `UserConstructionScript`
  (bind (_iteminfo_0_itemtype _iteminfo_0_itemname _iteminfo_0_itemimage _iteminfo_0_itemclass _iteminfo_0_itemindex _iteminfo_0_itemslot _iteminfo_0_itemamount) (break `/Game/Character/Interactables/Objects/FItemInfo` (`self.ItemInfo_0`)))
  (`parent.UserConstructionScript`)
  (set `self.ItemInfo_0` (make `/Game/Character/Interactables/Objects/FItemInfo` _iteminfo_0_itemtype _iteminfo_0_itemname _iteminfo_0_itemimage (`GameplayStatics.GetObjectClass` self) _iteminfo_0_itemindex _iteminfo_0_itemslot _iteminfo_0_itemamount)))