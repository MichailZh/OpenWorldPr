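; BP_HookArea is a volume actor that marks where the player character (TestFpp) may use a hook.
; Every Tick it casts player 0's character to TestFpp and polls whether its Box overlaps that character, rather than using overlap events.
; Inside, it sets CanHook; outside, it clears CanHook and IsHooking and calls StopCable every frame, so each instance writes these flags regardless of any other area.
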(event `self.ReceiveTick`
  (params (DeltaSeconds :type "Float (single-precision)"))
  (bind _newvar_0 (`self.NewVar_0`))
  (bind _astest_fpp (cast `/Game/Character/MainCharFPP/TestFpp` (`GameplayStatics.GetPlayerCharacter` 0)))
  (bind _output_get (set `self.NewVar_0` _astest_fpp))
  (if (`PrimitiveComponent.IsOverlappingActor` (`self.Box`) _output_get)
    (set `/Game/Character/MainCharFPP/TestFpp.CanHook?` true _newvar_0)
    (else
      (set `/Game/Character/MainCharFPP/TestFpp.CanHook?` false _newvar_0)
      (set `/Game/Character/MainCharFPP/TestFpp.IsHooking` false _newvar_0)
      (`/Game/Character/MainCharFPP/TestFpp.StopCable` _newvar_0))))

(fn `NewFunction_0`)

(fn `UserConstructionScript`)